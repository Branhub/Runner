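; Placeholder component in the runner's road assets that marks where an energy capsule can spawn on its owning actor.
; SpawnCapsule, not called within this file, draws a random config and, unless its energy is near zero, spawns an EnergyCapsule at the placeholder's relative transform, configures it and attaches it to the owner.
; GetRandomConfig makes a weighted pick from CapsuleTypes by possibility, so zero-energy entries act as empty slots.
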(fn `GetRandomConfig`
  (returns (result :type "/Game/Runner/Blueprint/CapsuleConfigs Structure"))
  (locals (possibilitySum :type Integer) (randomValue :type Integer) (tempSum :type Integer))
  (for _array_element (`self.capsuleTypes`)
    (set `local.possibilitySum` (+ (`.possibility_10_30C1C2554F5C84B59DD7B2B28DD69CE7` (break `/Game/Runner/Blueprint/CapsuleConfigs` _array_element)) (`local.possibilitySum`))))
  (set `local.randomValue` (`KismetMathLibrary.RandomIntegerInRange` 1 (`local.possibilitySum`)))
  (for _index (range (+ (`KismetArrayLibrary.Array_LastIndex` (`self.capsuleTypes`)) 1))
    (bind (_output_energy _output_color _output_possibility) (break `/Game/Runner/Blueprint/CapsuleConfigs` (`|GetArrayItem` (`self.capsuleTypes`) _index)))
    (bind _output_get (set `local.tempSum` (+ _output_possibility (`local.tempSum`))))
    (if (>= _output_get (`local.randomValue`))
      (return (make `/Game/Runner/Blueprint/CapsuleConfigs` _output_energy _output_color _output_possibility)))))

(fn `SpawnCapsule`
  (locals (possibilitySum :type Integer))
  (bind _result (`self.GetRandomConfig`))
  (if (not (`KismetMathLibrary.NearlyEqual_FloatFloat` (break `/Game/Runner/Blueprint/CapsuleConfigs` _result) 0.0 0.0001))
    (bind _returnvalue (`|SpawnActorFromClass` "/Game/Runner/Blueprint/EnergyCapsule.EnergyCapsule_C" (`self.GetRelativeTransform`) "Undefined" "OverrideRootScale" null null))
    (`/Game/Runner/Blueprint/EnergyCapsule.SetConfig` _returnvalue (make `/Game/Runner/Blueprint/CapsuleConfigs` (break `/Game/Runner/Blueprint/CapsuleConfigs` _result) (`.color_6_CB542E744F761B406EFF2AA0E43C72D9` (break `/Game/Runner/Blueprint/CapsuleConfigs` _result)) (`.possibility_10_30C1C2554F5C84B59DD7B2B28DD69CE7` (break `/Game/Runner/Blueprint/CapsuleConfigs` _result))))
    (`Actor.K2_AttachToActor` _returnvalue (`self.GetOwner`) "None" "KeepRelative" "KeepRelative" "KeepRelative" true)))