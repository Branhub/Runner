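; Road generator for a runner game that keeps a chain of road segments extending along X.
; BeginPlay spawns the InitRoads sequence end to end from each segment's End component, then seeds a random stream from clock milliseconds.
; RunnerLeveRoad appends a random RoadClasses segment, treating CurRoad as a ring buffer that destroys the oldest segment once RoadBufferSize is reached.
; PlayerInput and RunnerMove relay speeds and movement to every buffered segment.
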(event `self.ReceiveBeginPlay`
  (bind _initroads (`self.initRoads`))
  (bind _returnvalue (`|SpawnActorFromClass` (`|GetArrayItem` (`self.initRoads`)) (`KismetMathLibrary.MakeTransform` (0.0 0.0 0.0)) "Undefined" "OverrideRootScale" null 0 null))
  (bind _output_get (set `self.lastSpawnedRoad` _returnvalue))
  (bind _returnvalue_2 (`KismetArrayLibrary.Array_Add` (`self.curRoad`) _output_get))
  (set `self.newestRoadIndex` _returnvalue_2)
  (for _index (range 1 (`KismetArrayLibrary.Array_Length` _initroads))
    (bind _location (`self.CalStartLocation` (`self.lastSpawnedRoad`)))
    (bind _returnvalue_3 (`|SpawnActorFromClass` (`|GetArrayItem` _initroads _index) (`KismetMathLibrary.MakeTransform` _location) "Undefined" "OverrideRootScale" null _index null))
    (bind _output_get_2 (set `self.lastSpawnedRoad` _returnvalue_3))
    (bind _returnvalue_4 (`KismetArrayLibrary.Array_Add` (`self.curRoad`) _output_get_2))
    (set `self.newestRoadIndex` _returnvalue_4))
  (set `self.roadRandomStream` (`KismetMathLibrary.MakeRandomStream` (`KismetMathLibrary.GetMillisecond` (`KismetMathLibrary.Now`)))))

(event `PlayerInput`
  (params (xSpeed :type "Float (double-precision)") (zSpeed :type "Float (double-precision)"))
  (for _array_element (`self.curRoad`)
    (`|ExecutionSequence`
      (:`then_0`
        (set `/Game/Runner/Blueprint/Road/BaseRoad.xSpeed` xSpeed _array_element))
      (:`then_1`
        (set `/Game/Runner/Blueprint/Road/BaseRoad.zSpeed` zSpeed _array_element)))))

(event `RunnerMove`
  (params (runnerMoveLength :type "Float (double-precision)"))
  (for _array_element (`self.curRoad`)
    (`/Game/Runner/Blueprint/Road/BaseRoad.RunnerMove` _array_element runnerMoveLength)))

(event `RunnerLeveRoad`
  (params (index :type Integer))
  (bind _newparam (`self.GetRandomRoad`))
  (bind _location (`self.CalStartLocation` (`self.lastSpawnedRoad`)))
  (bind _returnvalue (`|SpawnActorFromClass` _newparam (`KismetMathLibrary.MakeTransform` _location) "Undefined" "OverrideRootScale" null 0 null))
  (bind _output_get (set `self.lastSpawnedRoad` _returnvalue))
  (if (< (`KismetArrayLibrary.Array_Length` (`self.curRoad`)) (`self.roadBufferSize`))
    (bind _returnvalue_2 (`KismetArrayLibrary.Array_Add` (`self.curRoad`) _output_get))
    (bind _output_get_2 (set `/Game/Runner/Blueprint/Road/BaseRoad.index` _returnvalue_2 _output_get))
    (set `self.newestRoadIndex` _output_get_2)
    (else
      (`self.K2_DestroyActor` (`|GetArrayItem` (`self.curRoad`) (`self.oldestRoadIndex`)))
      (bind _next (`self.GetNextCurRoadIndex` (`self.oldestRoadIndex`)))
      (set `self.oldestRoadIndex` _next)
      (bind _next_2 (`self.GetNextCurRoadIndex` (`self.newestRoadIndex`)))
      (bind _output_get_3 (set `self.newestRoadIndex` _next_2))
      (`KismetArrayLibrary.Array_Set` (`self.curRoad`) _output_get_3 _output_get))))

(fn `CalStartLocation`
  (params (lastRoad :type "/Game/Runner/Blueprint/Road/BaseRoad Object Reference"))
  (returns (location :type "Vector Structure"))
  (bind (_returnvalue_x _returnvalue_y _returnvalue_z) (`KismetMathLibrary.BreakVector` (`self.K2_GetActorLocation` lastRoad)))
  (return (`KismetMathLibrary.MakeVector` (+ (.x (.location (`SceneComponent.K2_GetComponentToWorld` (`/Game/Runner/Blueprint/Road/BaseRoad.End` lastRoad)))) (/ (* 64 (.x (.scale (`SceneComponent.K2_GetComponentToWorld` (`/Game/Runner/Blueprint/Road/BaseRoad.End` lastRoad))))) 2.0)) _returnvalue_y _returnvalue_z)))

(fn `GetNextCurRoadIndex`
  (params (cur :type Integer))
  (returns (next :type Integer))
  (locals (result :type Integer))
  (if (>= cur (`KismetArrayLibrary.Array_LastIndex` (`self.curRoad`)))
    (set `local.result` 0)
    (else
      (set `local.result` (+ (`local.cur`) 1))))
  (return (`local.result`)))

(fn `GetRandomRoad`
  (returns (NewParam :type "/Game/Runner/Blueprint/Road/BaseRoad Class Reference"))
  (return (`|GetArrayItem` (`self.roadClasses`) (`KismetMathLibrary.RandomIntegerFromStream` (`KismetArrayLibrary.Array_Length` (`self.roadClasses`)) (`self.roadRandomStream`)))))

(fn `SpawnNewRoad`
  (bind _newparam (`self.GetRandomRoad`))
  (bind _location (`self.CalStartLocation` (`self.lastSpawnedRoad`)))
  (bind _returnvalue (`|SpawnActorFromClass` _newparam (`KismetMathLibrary.MakeTransform` _location) "Undefined" "OverrideRootScale" null 0 null))
  (bind _output_get (set `self.lastSpawnedRoad` _returnvalue))
  (`KismetArrayLibrary.Array_Add` (`self.curRoad`) _output_get))

(fn `UserConstructionScript`)