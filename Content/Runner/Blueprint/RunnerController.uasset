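; RunnerController is the controller that routes player input to the RunnerCharacter pawn in a runner game.
; The move and jump action presses each cast the controlled pawn to RunnerCharacter, then call OnRunClick or RunnerJump on it.
; An unconnected leftover branch would pass the character's negated speed to the first Generater actor as horizontal input, but it never executes.
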(event `InputAction|move`
  (params (Key :type "Key Structure"))
  (:`Pressed`
    (bind _asrunner_character (cast `/Game/Runner/Blueprint/RunnerCharacter` (`self.K2_GetPawn`)))
    (`/Game/Runner/Blueprint/RunnerCharacter.OnRunClick` _asrunner_character)))

(event `InputAction|jump`
  (params (Key :type "Key Structure"))
  (:`Pressed`
    (bind _asrunner_character (cast `/Game/Runner/Blueprint/RunnerCharacter` (`self.K2_GetPawn`)))
    (`/Game/Runner/Blueprint/RunnerCharacter.RunnerJump` _asrunner_character)))

(fn `UserConstructionScript`)