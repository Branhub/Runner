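; Energy capsule pickup that changes a runner character's energy on overlap and then destroys itself.
; BeginPlay creates a dynamic material instance on the static mesh.
; SetConfig stores energy and color from a config and pushes the color into that material, so it relies on BeginPlay having run first.
; Mesh overlaps with anything other than a RunnerCharacter are ignored.
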(event `self.ReceiveBeginPlay`
  (bind _returnvalue (`PrimitiveComponent.CreateDynamicMaterialInstance` (`self.StaticMesh`) 0 null))
  (set `self.capsuleMaterialInst` _returnvalue))

(event `self.StaticMesh.OnComponentBeginOverlap`
  (params (OverlappedComponent :type "PrimitiveComponent Object Reference") (OtherActor :type "Actor Object Reference") (OtherComp :type "PrimitiveComponent Object Reference") (OtherBodyIndex :type Integer) (bFromSweep :type Boolean) (SweepResult :type "HitResult Structure (by ref)"))
  (bind _asrunner_character (cast `/Game/Runner/Blueprint/RunnerCharacter` OtherActor))
  (`/Game/Runner/Blueprint/RunnerCharacter.ChangeEnergy` _asrunner_character (`self.energy`))
  (`self.K2_DestroyActor`))

(fn `SetConfig`
  (params (config :type "/Game/Runner/Blueprint/CapsuleConfigs Structure"))
  (set `self.energy` config_energy_2_784A28F242F17540616B2E9D4A4B3524)
  (bind _output_get (set `self.color` config_color_6_CB542E744F761B406EFF2AA0E43C72D9))
  (`MaterialInstanceDynamic.SetVectorParameterValue` (`self.capsuleMaterialInst`) "capsuleColor" _output_get))

(fn `UserConstructionScript`)