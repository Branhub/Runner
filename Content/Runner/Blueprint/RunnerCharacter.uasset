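; Player character for a click-driven runner that creates its UI and spends energy to jump.
; Click intervals set acceleration, top speed and a timer that starts deceleration, so faster tapping runs faster but is harder to sustain.
; Tick integrates speed, changes energy while running and passes movement to the road Generater, so the road moves instead of the runner.
; Empty energy forces deceleration on click, and leaving a road's End component notifies the Generater.
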(event `self.ReceiveBeginPlay`
  (bind _returnvalue_x (`KismetMathLibrary.BreakVector` (`self.K2_GetActorLocation`)))
  (set `self.originX` _returnvalue_x)
  (set `self.curTopSpeed` (`self.defaultTopSpeed`))
  (bind _outactors (`GameplayStatics.GetAllActorsOfClass` "/Game/Runner/Blueprint/Road/Generater.Generater_C"))
  (set `self.roadGenerater` (`|GetArrayItem` _outactors))
  (set `self.curEnergy` (`self.defaultEnergy`))
  (set `self.curEnergyChangeSpeed` (`self.defaultEnergyChangeSpeed`))
  (bind _returnvalue (`|CreateWidget` "/Game/Runner/Blueprint/UI/UI.UI_C"))
  (bind _output_get (set `self.UIWidget` _returnvalue))
  (`UserWidget.AddToViewport` _output_get 0))

(event `self.ReceiveTick`
  (params (DeltaSeconds :type "Float (single-precision)"))
  (bind _roadgenerater (`self.roadGenerater`))
  (if (`|EnumEquality` (`self.curState`) "NewEnumerator1")
    (`self.ChangeEnergy` (* DeltaSeconds (`self.curEnergyChangeSpeed`))))
  (bind _output_get (set `self.curSpeed` (`KismetMathLibrary.FClamp` (+ (`self.curSpeed`) (* (`self.curAcc`) DeltaSeconds)) (`self.curMinSpeed`) (`self.curTopSpeed`))))
  (if (`KismetMathLibrary.NearlyEqual_FloatFloat` _output_get 0.0 0.0001)
    (`self.ResetWhenSpeedIsZero`)
    (else
      (set `self.curState` "NewEnumerator1")))
  (set `self.isInAir` (`NavMovementComponent.IsFalling` (`self.CharacterMovement`)))
  (`/Engine/EditorBlueprintResources/StandardMacros.IsValid` _roadgenerater
    (:`Is Valid`
      (`/Game/Runner/Blueprint/Road/Generater.RunnerMove` _roadgenerater (* (`self.curSpeed`) DeltaSeconds)))))

(event `OnRunClick`
  (`self.CalClickElapse`)
  (`self.CalAcc`)
  (`self.CalTopSpeed`))

(event `self.CapsuleComponent.OnComponentEndOverlap`
  (params (OverlappedComponent :type "PrimitiveComponent Object Reference") (OtherActor :type "Actor Object Reference") (OtherComp :type "PrimitiveComponent Object Reference") (OtherBodyIndex :type Integer))
  (bind _asbase_road (cast `/Game/Runner/Blueprint/Road/BaseRoad` OtherActor))
  (if (== (`/Game/Runner/Blueprint/Road/BaseRoad.End` _asbase_road) OtherComp)
    (`/Game/Runner/Blueprint/Road/Generater.RunnerLeveRoad` (`self.roadGenerater`) (`/Game/Runner/Blueprint/Road/BaseRoad.index` _asbase_road))))

(event `self.FloorTester.OnComponentBeginOverlap`
  (params (OverlappedComponent :type "PrimitiveComponent Object Reference") (OtherActor :type "Actor Object Reference") (OtherComp :type "PrimitiveComponent Object Reference") (OtherBodyIndex :type Integer) (bFromSweep :type Boolean) (SweepResult :type "HitResult Structure (by ref)"))
  ;[1 1 1] FloorTester碰到阻挡Pawn的物体，且该物体Z坐标比Runner的Z坐标低，就算落到地上（暂时不用）
)

(event `self.FloorTester.OnComponentEndOverlap`
  (params (OverlappedComponent :type "PrimitiveComponent Object Reference") (OtherActor :type "Actor Object Reference") (OtherComp :type "PrimitiveComponent Object Reference") (OtherBodyIndex :type Integer))
  ;[1 1 1] FloorTester和某个阻挡物脱离接触，好像也没什么需要做的（暂时不用）
)

(fn `CalAcc`
  (bind _elapsetolastclick (`self.elapseToLastClick`))
  (if (<= (`self.curEnergy`) 0.0)
    (if (`KismetSystemLibrary.K2_TimerExists` null "StartDec")
      (`KismetSystemLibrary.K2_ClearTimer` null "StartDec"))
    (`self.StartDec`)
    (elif (`self.firstClick`)
      ;[1 1 1] 从静止开始的第一次点击，会有一个默认加速时间
      (set `self.curAcc` (`self.defaultAcc`))
      (`KismetSystemLibrary.K2_SetTimerDelegate` (`|CreateDelegate` :!event `StartDec`) (`self.defaultAccTime`))
      (set `self.firstClick` false)
      (if (not (`NavMovementComponent.IsFalling` (`self.CharacterMovement`)))
        (set `self.curState` "NewEnumerator1"))
      (elif (not (`KismetMathLibrary.NearlyEqual_FloatFloat` (`self.curSpeed`) 0.0 0.0001))
        ;[1 1 1] 设置减速Timer，这样点的越快，要想不减速也就越难
        (`KismetSystemLibrary.K2_SetTimerDelegate` (`|CreateDelegate` :!event `StartDec`) (/ _elapsetolastclick 1000.0))
        ;[1 1 1] 设置加速度，点的越快，加速度越大
        (set `self.curAcc` (`KismetMathLibrary.FMin` (`self.maxAcc`) (+ (`self.defaultAcc`) (/ (`self.accDividend`) _elapsetolastclick))))))))

(fn `CalClickElapse`
  (locals (now :type "DateTime Structure"))
  (bind _returnvalue (`KismetMathLibrary.GetTotalMilliseconds` (- (`local.now`) (`self.lastClick`))))
  (set `local.now` (`KismetMathLibrary.Now`))
  (if (`KismetMathLibrary.NearlyEqual_FloatFloat` _returnvalue 0.0 0.1)
    (set `self.elapseToLastClick` 1.0)
    (else
      (set `self.elapseToLastClick` _returnvalue)))
  (set `self.lastClick` (`local.now`)))

(fn `CalTopSpeed`
  (set `self.curTopSpeed` (`KismetMathLibrary.FMin` (+ (`self.defaultTopSpeed`) (/ (`self.topspeedDividend`) (`self.elapseToLastClick`))) (`self.maxTopSpeed`))))

(fn `ChangeEnergy`
  (params (change :type "Float (double-precision)"))
  (set `self.curEnergy` (`KismetMathLibrary.FClamp` (+ change (`self.curEnergy`)) 0.0 (`self.maxEnergy`))))

(fn `FallToGround`
  (if (> (`self.curSpeed`) 0.0)
    (set `self.curState` "NewEnumerator1")
    (else
      (set `self.curState` "NewEnumerator0"))))

(fn `ResetWhenSpeedIsZero`
  (set `self.curSpeed` 0.0)
  (set `self.curAcc` 0.0)
  (set `self.firstClick` true)
  (set `self.curState` "NewEnumerator0")
  (if (`KismetSystemLibrary.K2_TimerExists` null "StartDec")
    (`KismetSystemLibrary.K2_ClearTimer` null "StartDec")))

(fn `RunnerJump`
  (bind _jumpenergy (`self.jumpEnergy`))
  (if (>= (`self.curEnergy`) (`KismetMathLibrary.Abs` _jumpenergy))
    (`self.ChangeEnergy` _jumpenergy)
    (`self.Jump`)))

(fn `StartDec`
  (if (>= (`self.curSpeed`) 0.0)
    (if (>= (`self.curSpeed`) (`self.curTopSpeed`))
      (set `self.curAcc` (`self.overspeedDec`))
      (else
        (set `self.curAcc` (`self.defaultDec`))))))

(fn `UpdateClickBuffer`
  (`/Engine/EditorBlueprintResources/StandardMacros.IncrementInt` (`self.totalClicks`)))

(fn `UserConstructionScript`)